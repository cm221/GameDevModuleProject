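; An interactable puzzle actor whose point light starts dark and lights up bright green when its condition is met.
; Three ActionByObjectInTriggerVolume sources each latch their own flag on ObjectFound, and the light turns on once all three are set.
; The OnInteract event turns the same light on directly, bypassing the flags, and nothing resets the flags or the light during play.
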(event `self.ReceiveBeginPlay`
  (`LightComponent.SetIntensity` (`self.PointLight`) 0.0))

(event `/Game/Blueprints/InteractInterface_BP.OnInteract`
  (`LightComponent.SetIntensity` (`self.PointLight`) 33333.0 :!label _label)
  (`LightComponent.SetLightColor` (`self.PointLight`) (struct :`R` 0.23503 :`G` 0.95 :`B` 0.453888 :`A` 1.0) true))

(event `self.ActionByObjectInTriggerVolume.ObjectFound`
  (bind _output_get (set `self.NewVar_0` true))
  (if (and _output_get (stale `self.ActionByObjectInTriggerVolume1.ObjectFound` _output_get) (stale `self.ActionByObjectInTriggerVolume2.ObjectFound` _output_get)) :!label _label_2
    (goto _label)))

(event `self.ActionByObjectInTriggerVolume1.ObjectFound`
  (bind _output_get (set `self.NewVar_1` true))
  (goto _label_2))

(event `self.ActionByObjectInTriggerVolume2.ObjectFound`
  (bind _output_get (set `self.NewVar_2` true))
  (goto _label_2))

(fn `UserConstructionScript`)