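; Level 1 door blueprint that swings open once three trigger volumes all detect their objects at the same time.
; Three ActionByObjectInTriggerVolume components set or clear a flag each as objects are found or lost.
; When all three flags are true, a DoOnce gate plays the DoorRotation timeline, which drives the door's relative yaw.
; Nothing resets the gate or reverses the timeline, so the door stays open.
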(event `self.ActionByObjectInTriggerVolume.ObjectFound`
  (bind _output_get (set `self.Object1InVol` true))
  (if (and _output_get (stale `self.ActionByObjectInTriggerVolume1.ObjectFound` _output_get) (stale `self.ActionByObjectInTriggerVolume2.ObjectFound` _output_get)) :!label _label
    (`/Engine/EditorBlueprintResources/StandardMacros.DoOnce` false
      (:`Completed`
        ;[1 1 1] Open door rotation
        (bind (_direction _doorrotation) (`Timeline|DoorRotation`)
          (:`Update`
            (`SceneComponent.K2_SetRelativeRotation` (`self.Door`) (`KismetMathLibrary.MakeRotator` 0.0 0.0 _doorrotation) false false)))))))

(event `self.ActionByObjectInTriggerVolume1.ObjectFound`
  (bind _output_get (set `self.Object2InVol` true))
  (goto _label))

(event `self.ActionByObjectInTriggerVolume2.ObjectFound`
  (bind _output_get (set `self.Object3InVol` true))
  (goto _label))

(event `self.ActionByObjectInTriggerVolume.ObjectNotFound`
  ;[1 1 1] When object not in volume
  (set `self.Object1InVol` false))

(event `self.ActionByObjectInTriggerVolume1.ObjectNotFound`
  ;[1 1 1] When object not in volume
  (set `self.Object2InVol` false))

(event `self.ActionByObjectInTriggerVolume2.ObjectNotFound`
  ;[1 1 1] When object not in volume
  (set `self.Object3InVol` false))

(fn `UserConstructionScript`)