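; Lever prop for Level 1 that toggles between on and off when interacted with and signals a linked secret door.
; OnInteract plays one of two swing timelines based on LeverOnState, driving the lever mesh's relative roll.
; Each timeline update, rather than a single trigger, calls ActivateSecretDoorMessage on SecretDoorRef with the target state.
; LeverOnState flips only when the swing finishes.
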(event `/Game/Blueprints/InteractInterface_BP.OnInteract`
  (bind _lever (`self.Lever`))
  ;[1 1 1] Rotate the lever from off & on position
  (if (`self.LeverOnState`)
    (bind (_direction _leverswing) (`Timeline|LeverSwingToOff` :!via `PlayFromStart`)
      (:`Update`
        (`SceneComponent.K2_SetRelativeRotation` _lever (`KismetMathLibrary.MakeRotator` _leverswing) false false)
        (message `/Game/Props/Level1/Blueprints/SecretDoorInterface.ActivateSecretDoor` (`self.SecretDoorRef`) false))
      (:`Finished`
        (set `self.LeverOnState` false)))
    (else
      (bind (_direction_2 _leverswing_2) (`Timeline|LeverSwingToOn` :!via `PlayFromStart`)
        (:`Update`
          (`SceneComponent.K2_SetRelativeRotation` _lever (`KismetMathLibrary.MakeRotator` _leverswing_2) false false)
          (message `/Game/Props/Level1/Blueprints/SecretDoorInterface.ActivateSecretDoor` (`self.SecretDoorRef`) true))
        (:`Finished`
          (set `self.LeverOnState` true))))))

(fn `UserConstructionScript`)