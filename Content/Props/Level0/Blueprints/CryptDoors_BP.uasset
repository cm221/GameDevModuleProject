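; Crypt double door in Level0 that opens once and serves as the exit to Level1.
; When the ActionByObjectInTriggerVolume component reports ObjectFound, a DoOnce gate plays the DoorRotation timeline, which sets the yaw of both doors.
; Each timeline update also looks up all CemetaryKey_BP actors and destroys the first, without checking that one exists.
; When the timeline finishes, it loads Level1 by name.
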(event `self.ActionByObjectInTriggerVolume.ObjectFound`
  (`/Engine/EditorBlueprintResources/StandardMacros.DoOnce` false
    (:`Completed`
      (bind (_direction _leftdoorrotation _rightdoorrotation) (`Timeline|DoorRotation`)
        (:`Update`
          (bind _outactors (`GameplayStatics.GetAllActorsOfClass` "/Game/Props/Level0/Blueprints/CemetaryKey_BP.CemetaryKey_BP_C"))
          (`self.K2_DestroyActor` (`KismetArrayLibrary.Array_Get` _outactors))
          (`SceneComponent.K2_SetRelativeRotation` (`self.LeftDoor`) (`KismetMathLibrary.MakeRotator` 0.0 0.0 _leftdoorrotation) false false)
          (`SceneComponent.K2_SetRelativeRotation` (`self.RightDoor`) (`KismetMathLibrary.MakeRotator` 0.0 0.0 _rightdoorrotation) false false))
        (:`Finished`
          (`GameplayStatics.OpenLevel` "Level1"))))))

(fn `UserConstructionScript`)