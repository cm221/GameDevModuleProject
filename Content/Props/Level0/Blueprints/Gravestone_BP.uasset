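; Gravestone prop Blueprint in Level0 that opens a gravestone UI screen when the player interacts with it.
; On interact it shows the mouse cursor and creates the Level0_Gravestone1 widget once, caching the reference for later uses.
; It then switches input to UI-only focused on that widget, adds it to the viewport and pauses the game.
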(event `/Game/Blueprints/InteractInterface_BP.OnInteract`
  (bind _gravestone_ui_1_ref (`self.Gravestone UI 1 Ref`))
  ;[1 1 1] Display Gravestone widget when user interacts
  (set `PlayerController.bShowMouseCursor` true (`GameplayStatics.GetPlayerController` 0))
  (`/Engine/EditorBlueprintResources/StandardMacros.IsValid` (`self.Gravestone UI 1 Ref`)
    (:`Is Valid`
      _)
    (:`Is Not Valid`
      (bind _returnvalue (`|CreateWidget` "/Game/UI/Level0/Level0_Gravestone1_BP.Level0_Gravestone1_BP_C"))
      (set `self.Gravestone UI 1 Ref` _returnvalue)))
  (`WidgetBlueprintLibrary.SetInputMode_UIOnlyEx` (`GameplayStatics.GetPlayerController` 0) _gravestone_ui_1_ref)
  (`UserWidget.AddToViewport` _gravestone_ui_1_ref 0)
  (`GameplayStatics.SetGamePaused` true))

(fn `UserConstructionScript`)