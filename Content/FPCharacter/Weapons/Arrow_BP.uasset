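; Arrow projectile that ignores the player character and, on hit, capsule-traces forward to resolve the impact.
; A bone hit applies damage, stops the arrow and attaches a spawned static arrow to that bone with a blood emitter.
; Particle collisions from that emitter spawn randomized, fading blood splatter decals.
; Other impacts swap the projectile for a static arrow flagged for pending destruction.
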(event `self.ObjectHit`
  (bind _collisionmesh (`self.CollisionMesh`))
  (bind _returnvalue (`SceneComponent.K2_GetComponentLocation` _collisionmesh))
  ;[1 1 1] Capsule trace when object is hit by projectile
  (bind (_outhit _returnvalue_2) (`KismetSystemLibrary.CapsuleTraceSingle_NEW` _returnvalue (+ _returnvalue (* (`KismetMathLibrary.GetForwardVector` (`SceneComponent.K2_GetComponentRotation` _collisionmesh)) 100.0)) 0.0 0.0 "TraceTypeQuery1"))
  (if _returnvalue_2
    (bind (_bblockinghit _binitialoverlap _time _location _impactpoint _normal _impactnormal _physmat _hitactor _hitcomponent _hitbonename) (`GameplayStatics.BreakHitResult` _outhit))
    ;[1 1 1] Comment
    (if (!= _hitbonename "None")
      ;[1 1 1] Apply damage to actor that was hit
      (`GameplayStatics.ApplyDamage` _hitactor (`self.ProjectileDamage`) (`GameplayStatics.GetPlayerController` 0) self "/Script/GameDevGroupModule.ProjectileDamageType")
      ;[1 1 1] Stop moving arrow, delete & attach static arrow to the model hit on the correct bone
      (`MovementComponent.StopMovementImmediately` (`self.ProjectileMovement`))
      (`self.K2_SetActorLocation` _impactpoint)
      (bind _returnvalue_3 (`|SpawnActorFromClass` "/Game/FPCharacter/Weapons/StaticArrow_BP.StaticArrow_BP_C" (`self.GetTransform` self) "Undefined" "OverrideRootScale"))
      (`self.K2_AttachToComponent` _returnvalue_3 _hitcomponent _hitbonename "KeepWorld" "KeepWorld" "KeepWorld" true)
      (bind _returnvalue_4 (`GameplayStatics.SpawnEmitterAtLocation` "/Game/BloodEffects/BloodParticles_P.BloodParticles_P" _impactpoint))
      (add `ParticleSystemComponent.OnParticleCollide` _returnvalue_4 (delegate `On Collide Event`))
      (else
        ;[1 1 1] Called if object collided with not model with bones & so static arrow createad & Pending Destoy called so arrow can be deleted
        (`MovementComponent.StopMovementImmediately` (`self.ProjectileMovement`) :!label _label)
        (bind _returnvalue_5 (`|SpawnActorFromClass` "/Game/FPCharacter/Weapons/StaticArrow_BP.StaticArrow_BP_C" (`self.GetTransform` self) "Undefined" "OverrideRootScale"))
        (`self.K2_DestroyActor`)
        (`/Game/FPCharacter/Weapons/StaticArrow_BP.PendingDestoy` _returnvalue_5)))
    (else
      (goto _label))))

(event `On Collide Event`
  (params (EventName :type Name) (EmitterTime :type "Float (double-precision)") (ParticleTime :type Integer) (Location :type "Vector Structure") (Velocity :type "Vector Structure") (Direction :type "Vector Structure") (Normal :type "Vector Structure") (BoneName :type Name))
  (bind _splatterlifespan (`self.SplatterLifeSpan`))
  ;[1 1 1] Blood decal splatter when blood particles collide
  (bind _returnvalue (`KismetMaterialLibrary.CreateDynamicMaterialInstance` "/Game/BloodEffects/BloodDecal_M.BloodDecal_M"))
  (`MaterialInstanceDynamic.SetScalarParameterValue` _returnvalue "BloodFrame" (`KismetMathLibrary.Conv_IntToDouble` (`KismetMathLibrary.RandomInteger` 11)))
  (bind _returnvalue_2 (`GameplayStatics.SpawnDecalAtLocation` _returnvalue (`KismetMathLibrary.Conv_DoubleToVector` (`KismetMathLibrary.RandomFloatInRange` 10.0 50.0)) Location (`KismetMathLibrary.Conv_VectorToRotator` (* Normal -1.0)) _splatterlifespan))
  (`DecalComponent.SetFadeOut` _returnvalue_2 (* _splatterlifespan 0.8) (* _splatterlifespan 0.2) true))

(event `self.ReceiveBeginPlay`
  ;[1 1 1] Ignore collisions with player capsule
  (`PrimitiveComponent.IgnoreActorWhenMoving` (`self.CollisionMesh`) (`GameplayStatics.GetPlayerCharacter` 0) true))

(fn `UserConstructionScript`)