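; Static crossbow arrow actor that produces blood effects and removes itself two seconds after its destroy event is called.
; On its spawn event it emits blood particles at the spawn location and binds to their collisions.
; Each collision spawns a randomly sized decal facing into the surface, using a dynamic material instance to pick a random splatter frame.
; Decals fade out over the last fifth of the splatter lifespan.
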(event `PendingDestoy`
  ;[1 1 1] When called destorys actor after set time
  (`KismetSystemLibrary.Delay` 2.0)
  (`self.K2_DestroyActor`))

(event `On Arrow Spawn`
  (bind _returnvalue (`GameplayStatics.SpawnEmitterAtLocation` "/Game/BloodEffects/BloodParticles_P.BloodParticles_P" (`self.Spawn Location`)))
  (add `ParticleSystemComponent.OnParticleCollide` _returnvalue (delegate `On Collide Event`)))

(event `On Collide Event`
  (params (EventName :type Name) (EmitterTime :type "Float (double-precision)") (ParticleTime :type Integer) (Location :type "Vector Structure") (Velocity :type "Vector Structure") (Direction :type "Vector Structure") (Normal :type "Vector Structure") (BoneName :type Name))
  (bind _splatter_life_span (`self.Splatter Life Span`))
  ;[1 1 1] Blood decal splatter when blood particles collide
  (bind _returnvalue (`KismetMaterialLibrary.CreateDynamicMaterialInstance` "/Game/BloodEffects/BloodDecal_M.BloodDecal_M"))
  (`MaterialInstanceDynamic.SetScalarParameterValue` _returnvalue "BloodFrame" (`KismetMathLibrary.Conv_IntToDouble` (`KismetMathLibrary.RandomInteger` 11)))
  (bind _returnvalue_2 (`GameplayStatics.SpawnDecalAtLocation` _returnvalue (`KismetMathLibrary.Conv_DoubleToVector` (`KismetMathLibrary.RandomFloatInRange` 10.0 50.0)) Location (`KismetMathLibrary.Conv_VectorToRotator` (* Normal -1.0)) _splatter_life_span))
  (`DecalComponent.SetFadeOut` _returnvalue_2 (* _splatter_life_span 0.8) (* _splatter_life_span 0.2) true))

(fn `UserConstructionScript`)