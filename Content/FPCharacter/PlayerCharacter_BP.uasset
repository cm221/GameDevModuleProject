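; Player character Blueprint that handles object interaction, the interact prompt and opening the pause menu.
; A looping timer polls GetInteractionObjectInReach, defined outside these graphs, and toggles the interact prompt flag on HUD_BP, found by widget class lookup.
; The Interact input repeats that reach check and sends OnInteractMessage to the object found.
; The Quit input creates and caches PauseMenu_BP, switches to UI-only input with cursor and pauses the game.
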(event `InputAction|Quit`
  (params (Key :type "Key Structure" :default "AnyKey"))
  (bind _pausemenureference (`self.PauseMenuReference`))
  ;[1 1 1] Open Pause Menu
  (:`Pressed`
    (set `PlayerController.bShowMouseCursor` true (`GameplayStatics.GetPlayerController` 0))
    (`/Engine/EditorBlueprintResources/StandardMacros.IsValid` (`self.PauseMenuReference`)
      (:`Is Valid`
        _)
      (:`Is Not Valid`
        (bind _returnvalue (`|CreateWidget` "/Game/UI/PauseMenu_BP.PauseMenu_BP_C"))
        (set `self.PauseMenuReference` _returnvalue)))
    (`WidgetBlueprintLibrary.SetInputMode_UIOnlyEx` (`GameplayStatics.GetPlayerController` 0) _pausemenureference)
    (`UserWidget.AddToViewport` _pausemenureference 0)
    (`GameplayStatics.SetGamePaused` true)))

(event `InteractTextDisplay`
  ;[1 1 1] Displays interact text on player's screen when interaction object subclass is in raycast
  (`self.GetInteractionObjectInReach`)
  (if (`self.ConfirmedInteractionObjectInReach`)
    (bind _foundwidgets (`WidgetBlueprintLibrary.GetAllWidgetsOfClass` "/Game/UI/HUD_BP.HUD_BP_C" false))
    (bind _ashud_bp (cast `/Game/UI/HUD_BP` (`KismetArrayLibrary.Array_Get` _foundwidgets)))
    (set `/Game/UI/HUD_BP.VisibleInteract` true _ashud_bp)
    (else
      (bind _foundwidgets_2 (`WidgetBlueprintLibrary.GetAllWidgetsOfClass` "/Game/UI/HUD_BP.HUD_BP_C" false))
      (bind _ashud_bp_2 (cast `/Game/UI/HUD_BP` (`KismetArrayLibrary.Array_Get` _foundwidgets_2)))
      (set `/Game/UI/HUD_BP.VisibleInteract` false _ashud_bp_2))))

(event `self.ReceiveBeginPlay`
  ;[1 1 1] Sets up loop of how often to raytrace & display interact text
  (`KismetSystemLibrary.K2_SetTimer` null "InteractTextDisplay" 0.2 true))

(event `InputAction|Interact`
  (params (Key :type "Key Structure" :default "AnyKey"))
  ;[1 1 1] When a key is pressed raycast to check if object can be interacted with & trigger On Interact event
  (:`Pressed`
    (bind _returnvalue (`self.GetInteractionObjectInReach`))
    (if (`self.ConfirmedInteractionObjectInReach`)
      (message `/Game/Blueprints/InteractInterface_BP.OnInteract` _returnvalue))))

(fn `UserConstructionScript`)